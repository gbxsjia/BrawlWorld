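; Player controller that drives a BasicCharacter with world-axis movement input and mouse aiming.
; It caches the controlled pawn on BeginPlay and forwards both movement axes to its InputMove.
; After the first left click, Tick traces WorldStatic under the cursor to update a flattened aim direction and accumulate an aim timer.
; Releasing the button resets the timer and passes the direction to FireInput, but never clears the aim flag.
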(event EventTick
  (params (DeltaSeconds :type Float%20%28single-precision%29))
  (bind _array (Utilities|Array|MakeArray "ObjectTypeQuery1"))
  (bind _controlcharacter (Variables|Default|GetControlCharacter))
  (bind (_hitresult _returnvalue) (Class|PlayerController|GetHitResultUnderCursorforObjects _array true))
  (bind _returnvalue_2 (Transformation|GetActorLocation _controlcharacter))
  (bind _location (Collision|BreakHitResult _hitresult))
  (bind _returnvalue_3 (- _location _returnvalue_2))
  (if (Variables|Default|GetAimInput)
    (if _returnvalue
      (Variables|Default|SetAimDirection (Math|Vector|Normalize (Math|Vector|MakeVector (.x _returnvalue_3) (.y _returnvalue_3) 0.0)))
      (Variables|Default|SetAimTimer (+ (Variables|Default|GetAimTimer) (Utilities|Time|GetWorldDeltaSeconds))))))

(event EventBeginPlay
  (bind _asbasic_character (Utilities|Casting|CastToBasicCharacter (Pawn|GetControlledPawn)))
  (Variables|Default|SetControlCharacter _asbasic_character))

(event Input|AxisEvents|InputAxisHorizontalMove
  (params (AxisValue :type Float%20%28single-precision%29))
  (Default|InputMove (Variables|Default|GetControlCharacter) (* (Class|KismetMathLibrary|VectorRight) AxisValue)))

(event Input|AxisEvents|InputAxisVerticalMove
  (params (AxisValue :type Float%20%28single-precision%29))
  (Default|InputMove (Variables|Default|GetControlCharacter) (* (Class|KismetMathLibrary|VectorForward) AxisValue)))

(event Input|MouseEvents|LeftMouseButton
  (params (Key :type Key%20Structure :default "None"))
  (:Pressed
    (Variables|Default|SetAimInput true))
  (:Released
    (Variables|Default|SetAimTimer 0.0)
    (Default|FireInput (Variables|Default|GetControlCharacter) (Variables|Default|GetAimDirection))))

(fn ConstructionScript)